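; WeaponHolder is a scene component that manages a list of held weapon classes and the single weapon actor currently equipped.
; It equips the first entry on BeginPlay, and next and previous calls cycle the index with wraparound.
; Each switch destroys the old actor, spawns the new class attached to the component and updates the display name.
; Trigger and scope calls pass through to the current weapon, with scoping state tracked on the holder.
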(event EventBeginPlay
  (CallFunction|EquipbyIndex))

(fn Equip
  (params (Weapon :type Weapon%20Class%20Reference))
  (Utilities|IsValid (Variables|Default|GetWeapon)
    (:Is%20Valid
      (Actor|DestroyActor (Variables|Default|GetWeapon))
      (Variables|Default|SetWeapon 0))
    (:Is%20Not%20Valid
      _))
  (bind _returnvalue (Game|SpawnActorfromClass Weapon (Transformation|GetWorldTransform) "Undefined" 0 0))
  (bind _output_get (Variables|Default|SetWeapon _returnvalue))
  (Transformation|AttachComponentToComponent _output_get self "None" "SnapToTarget" "SnapToTarget" "SnapToTarget" true)
  (Variables|Default|SetWeaponName (Utilities|Text|ToText(String) (Utilities|GetDisplayName _output_get))))

(fn NextWeapon
  (bind _result (Math|Integer|IncrementInt (Variables|Default|GetIndex))
    (:%20%20
      (CallFunction|EquipbyIndex (select (>= _result (Utilities|Array|Length (Variables|Default|GetWeaponTypesHeld))) 0 _result)))))

(fn PrevWeapon
  (bind _result (Math|Integer|DecrementInt (Variables|Default|GetIndex))
    (:%20%20
      (CallFunction|EquipbyIndex (select (< _result 0) (- (Utilities|Array|Length (Variables|Default|GetWeaponTypesHeld)) 1) _result)))))

(fn EquipbyIndex
  (params (Index :type Integer))
  (bind _weapontypesheld (Variables|Default|GetWeaponTypesHeld))
  (if (Utilities|Array|IsValidIndex _weapontypesheld Index)
    (Variables|Default|SetIndex Index)
    (CallFunction|Equip (Utilities|Array|Get(acopy) _weapontypesheld Index))))

(fn ScopeStart
  (Default|ScopeBegin (Variables|Default|GetWeapon))
  (Variables|Default|SetisScoping true))

(fn ScopeEnd
  (Default|ScopeEnd (Variables|Default|GetWeapon))
  (Variables|Default|SetisScoping false))

(fn TriggerPull
  (params (player :type Jetpack%20Character%20Object%20Reference))
  (Default|TriggerPull (Variables|Default|GetWeapon) player))

(fn TriggerRelease
  (Default|TriggerRelease (Variables|Default|GetWeapon)))