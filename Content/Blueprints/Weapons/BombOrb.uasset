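; BombOrb is a weapon Blueprint whose ability teleports the player to a projectile already in the world.
; AbilityCall finds the first actor of ProjectileType, moves player character 0 to its location with zero rotation, plays a teleport sound and destroys it.
; With no valid projectile, it only plays a click sound at the world origin.
; DestroyProjectiles is an empty stub, and a second click sound is never run.
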(fn ConstructionScript
  (|CallParentFunction))

(fn AbilityCall
  (bind _returnvalue (Game|GetPlayerCharacter 0))
  (bind _outactors (Actor|GetAllActorsOfClass (Variables|Default|GetProjectileType)))
  (Utilities|IsValid (Utilities|Array|Get(acopy) _outactors)
    (:Is%20Valid
      (Transformation|Teleport _returnvalue (Transformation|GetActorLocation (Utilities|Array|Get(acopy) _outactors)) "0, 0, 0")
      (Audio|PlaySoundatLocation "/Engine/VREditor/Sounds/VR_teleport_Cue.VR_teleport_Cue" (Transformation|GetActorLocation _returnvalue) "0, 0, 0" 1.0 1.0 0.0 0 0 0)
      (Actor|DestroyActor (Utilities|Array|Get(acopy) _outactors)))
    (:Is%20Not%20Valid
      (Audio|PlaySoundatLocation "/Engine/VREditor/Sounds/VR_click1_Cue.VR_click1_Cue" "0, 0, 0" "0, 0, 0" 1.0 1.0 0.0 0 0 0))))

(fn DestroyProjectiles
  (params (ActorClass :type Actor%20Class%20Reference)))